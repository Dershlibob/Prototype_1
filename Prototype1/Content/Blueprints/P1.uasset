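; P1 is the first player's character in a local two-player setup, tethered to a Handcuffs actor.
; Its own input axes drive movement relative to control rotation, while P2 axes are forwarded to P2 actors found by class lookup.
; Each Tick looks up Handcuffs and snaps the capsule back to its last saved position when it strays beyond a fixed distance, otherwise saving the current one.
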(event `InputAxis|Forward/Back(P1)`
  (params (AxisValue :type "Float (single-precision)"))
  (`self.AddMovementInput` (`KismetMathLibrary.GetForwardVector` (`self.GetControlRotation`)) AxisValue))

(event `InputAxis|Left/Right(P1)`
  (params (AxisValue :type "Float (single-precision)"))
  (`self.AddMovementInput` (`KismetMathLibrary.GetRightVector` (`self.GetControlRotation`)) AxisValue))

(event `self.ReceiveTick`
  (params (DeltaSeconds :type "Float (single-precision)"))
  (bind _capsulecomponent (`self.CapsuleComponent`))
  (bind _returnvalue (`SceneComponent.K2_GetComponentLocation` _capsulecomponent))
  (bind _outactors (`GameplayStatics.GetAllActorsOfClass` "/Game/Blueprints/Handcuffs.Handcuffs_C"))
  (for _array_element _outactors
    _)
  (if (> (`KismetMathLibrary.VSize` (- (`SceneComponent.K2_GetComponentLocation` (`Actor.RootComponent` _array_element)) _returnvalue)) 100.0)
    (`SceneComponent.K2_SetWorldLocation` _capsulecomponent (stale _output_get) false false)
    (else
      (bind _output_get (set `self.PrevPosition` _returnvalue)))))

(event `InputAxis|Forward/Back(P2)`
  (params (AxisValue :type "Float (single-precision)"))
  (bind _outactors (`GameplayStatics.GetAllActorsOfClass` "/Game/Blueprints/P2.P2_C"))
  (`/Game/Blueprints/P1-to-P2-interface.P2(Up/Down)` _outactors AxisValue))

(event `InputAxis|Left/Right(P2)`
  (params (AxisValue :type "Float (single-precision)"))
  (bind _outactors (`GameplayStatics.GetAllActorsOfClass` "/Game/Blueprints/P2.P2_C"))
  (`/Game/Blueprints/P1-to-P2-interface.P2(Left/Right)` _outactors AxisValue))

(fn `UserConstructionScript`)