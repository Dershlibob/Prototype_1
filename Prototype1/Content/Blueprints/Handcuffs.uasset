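; Handcuffs actor that follows a P1 actor by moving its DefaultSceneRoot1 component every frame.
; On Tick it gets all P1 actors and loops over them with an empty body, then uses the last array element.
; It teleport-free sets the component 100 units along that actor's capsule right vector, without sweep, and prints the position for debugging.
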(event `self.ReceiveTick`
  (params (DeltaSeconds :type "Float (single-precision)"))
  (bind _outactors (`GameplayStatics.GetAllActorsOfClass` "/Game/Blueprints/P1.P1_C"))
  (for _array_element _outactors
    _)
  (bind _capsulecomponent (`Character.CapsuleComponent` _array_element))
  (bind _returnvalue (+ (`SceneComponent.K2_GetComponentLocation` _capsulecomponent) (* (`SceneComponent.GetRightVector` _capsulecomponent) 100)))
  (`SceneComponent.K2_SetWorldLocation` (`self.DefaultSceneRoot1`) _returnvalue false false)
  (`KismetSystemLibrary.PrintString` (`KismetStringLibrary.Conv_VectorToString` _returnvalue)))

(fn `UserConstructionScript`)