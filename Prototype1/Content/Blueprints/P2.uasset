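; P2 is the second player's character, kept on a short leash to a Handcuffs actor in the level.
; Its own Up/Down and Left/Right axes drive movement relative to the control rotation.
; Each tick it finds the Handcuffs actors, measures the capsule's distance to the last one, and snaps back to its saved position when beyond a fixed radius, otherwise saving the current position.
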(event `/Game/Blueprints/P1-to-P2-interface.P2(Up/Down)`
  (params (`Axis Value` :type "Float (single-precision)"))
  (`self.AddMovementInput` (`KismetMathLibrary.GetForwardVector` (`self.GetControlRotation`)) `Axis Value`))

(event `self.ReceiveTick`
  (params (DeltaSeconds :type "Float (single-precision)"))
  (bind _capsulecomponent (`self.CapsuleComponent`))
  (bind _returnvalue (`SceneComponent.K2_GetComponentLocation` _capsulecomponent))
  (bind _outactors (`GameplayStatics.GetAllActorsOfClass` "/Game/Blueprints/Handcuffs.Handcuffs_C"))
  (for _array_element _outactors
    _)
  (if (> (`KismetMathLibrary.VSize` (- (`SceneComponent.K2_GetComponentLocation` (`Actor.RootComponent` _array_element)) _returnvalue)) 100.0)
    (`SceneComponent.K2_SetWorldLocation` _capsulecomponent (stale _output_get) false false)
    (else
      (bind _output_get (set `self.Prev Position` _returnvalue)))))

(event `/Game/Blueprints/P1-to-P2-interface.P2(Left/Right)`
  (params (`Axis Value` :type "Float (single-precision)"))
  (`self.AddMovementInput` (`KismetMathLibrary.GetRightVector` (`self.GetControlRotation`)) `Axis Value`))

(fn `UserConstructionScript`)